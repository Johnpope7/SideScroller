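; Paper2D side-scrolling player character with horizontal movement, double jump and flipbook animation.
; MoveRight input moves along X, flips control yaw to face the travel direction and triggers the animation update.
; A DoN gate allows two upward LaunchCharacter jumps until landing resets it.
; The AnimationStateMachine function uses falling and velocity checks in two macros to select the idle, running or jumping flipbook.
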(event `self.ReceiveBeginPlay`
  ;[1 1 1] Replication (For Multiplayer)
  (`ActorComponent.SetIsReplicated` (`self.Sprite`) false))

(event `InputAxis|MoveRight`
  (params (AxisValue :type "Float (single-precision)"))
  ;[1 1 1] Horizontal Movement
  (`self.AddMovementInput` (1.0 0.0 0.0) AxisValue)
  (`self.UpdateAnimation`)
  (`/Engine/EditorBlueprintResources/StandardMacros.CompareFloat` AxisValue
    (:`>`
      (`Controller.SetControlRotation` (`self.GetController`) (`KismetMathLibrary.MakeRotator` 0.0)))
    (:`<`
      (`Controller.SetControlRotation` (`self.GetController`) (`KismetMathLibrary.MakeRotator` 0.0 0.0 180.0)))))

(event `InputAction|Jump`
  (params (Key :type "Key Structure"))
  ;[1 1 1] Jump Handling
  (:`Pressed`
    (bind _counter (`/Engine/EditorBlueprintResources/StandardMacros.Do N` 2 :!label _label)
      (:`Exit`
        (switch `int` _counter
          (:`1`
            (`self.LaunchCharacter` (0.0 0.0 1000.0)))
          (:`2`
            (`self.LaunchCharacter` (0.0 0.0 1000.0))))))))

(event `UpdateAnimation`
  ;[1 1 1] Animation Handling
  (set `self.IsMoving` (> (`KismetMathLibrary.VSize` (`self.GetVelocity`)) 0.0))
  (set `self.IsFalling` (`NavMovementComponent.IsFalling` (`self.CharacterMovement`)))
  (bind _output_flipbook (`self.AnimationStateMachine` (`self.IsFalling`) (`self.IsMoving`)))
  (`PaperFlipbookComponent.SetFlipbook` (`self.Sprite`) _output_flipbook))

(event `self.OnLanded`
  (params (Hit :type "HitResult Structure (by ref)"))
  ;[1 1 1] Jump Handling
  (goto _label :!via `Reset`))

(fn `AnimationStateMachine`
  (params (IsFalling :type Boolean) (IsMoving :type Boolean))
  (returns (`Output Flipbook` :type "PaperFlipbook Object Reference"))
  (locals (AnimationState :type "/Game/Game/Data/AnimationState Enum") (IsFallingLocal :type Boolean) (IsMovingLocal :type Boolean))
  ;[1 1 1] Collect Data
  (set `local.IsFallingLocal` IsFalling)
  (set `local.IsMovingLocal` IsMoving)
  ;[1 1 1] Test Movement Data
  (if (`local.IsFallingLocal`)
    ;[1 1 1] Set AnimationState
    (set `local.AnimationState` "NewEnumerator2")
    (elif (`local.IsMovingLocal`)
      (set `local.AnimationState` "NewEnumerator1")
      (else
        (set `local.AnimationState` "NewEnumerator0"))))
  (return (select `/Game/Game/Data/AnimationState` (`local.AnimationState`) :`NewEnumerator0` (`self.IdleFlipbook`) :`NewEnumerator1` (`self.RunFlipbook`) :`NewEnumerator2` (`self.JumpFlipbook`))))

(fn `UserConstructionScript`)